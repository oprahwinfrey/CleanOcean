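; BP_Trash is a data-driven trash actor that can be sucked into a vacuum and carries a score.
; Its construction script reads a data table row to set mesh, score, mass override and vacuum requirement, showing error text if the row is missing.
; MoveToTargetAndSelfDestroy handles the final suction step: it disables physics and collision, then scales the actor by a timeline while moving the mesh to the target before destroying itself.
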(event Custom|MoveToTargetAndSelfDestroy
  (params (targetPoint :type Vector))
  (bind _static_mesh (Variables|Default|GetStatic%20mesh))
  ;[1 1 1] Reach target and destroy (At this point, its in the vaccuum last step)
  (Physics|SetSimulatePhysics (Variables|Default|GetStatic%20mesh) false)
  (Collision|SetCollisionEnabled (Variables|Default|GetStatic%20mesh) "NoCollision")
  (Utilities|FlowControl|Sequence
    (:then_0
      (bind _1_to_0_in_0_1 (Timeline|Timeline PlayFromStart)
        (:Update
          (Transformation|SetActorScale3D (Math|Conversions|ToVector(Float) _1_to_0_in_0_1)))))
    (:then_1
      (Components|MoveComponentTo _static_mesh targetPoint (Variables|/Script/Engine.SceneComponent|GetRelativeRotation _static_mesh) false false 0.1 false)
      (Actor|DestroyActor))))

(fn ConstructionScript
  (bind _objecttobecreated (Variables|Default|GetObjectToBeCreated))
  (bind _returnvalue (Utilities|GetDataTableRow (.datatable _objecttobecreated) (.rowname _objecttobecreated))
    (:then
      (|Setproperties _returnvalue))
    (:RowNotFound
      (Development|PrintString "Could not create the BP_Trash from data table row.")
      (Rendering|SetVisibility (Variables|Default|GeterrorTextRender) true false))))