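; BP_Trash is a trash object that can be sucked up by a vacuum, configured per instance from a data table row.
; The construction script copies the row's mesh, size, scoring, mass and score required for vacuuming, and shows an error text if the row is missing.
; MoveToTargetAndSelfDestroy is the final suction step: it disables physics and collision, pulls the mesh to the target, hides the actor and destroys it after a delay.
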(event Custom|MoveToTargetAndSelfDestroy
  (params (target :type Vector))
  ;[1 1 1] Reach target and destroy (At this point, its in the vaccuum last step)
  (Physics|SetSimulatePhysics (Variables|Default|GetStatic%20mesh) false)
  (Collision|SetCollisionEnabled (Variables|Default|GetStatic%20mesh) "NoCollision")
  (Components|MoveComponentTo (Variables|Default|GetStatic%20mesh) target "0, 0, 0" false false 0.1 false)
  (Rendering|SetActorHiddenInGame true)
  (Utilities|FlowControl|Delay 5.0)
  (Actor|DestroyActor))

(fn ConstructionScript
  (bind _objecttobecreated (Variables|Default|GetObjectToBeCreated))
  (bind _returnvalue (Utilities|GetDataTableRow (.datatable _objecttobecreated) (.rowname _objecttobecreated))
    (:then
      (|Setproperties _returnvalue))
    (:RowNotFound
      (Development|PrintString "Could not create the BP_Trash from data table row.")
      (Rendering|SetVisibility (Variables|Default|GeterrorTextRender) true false))))